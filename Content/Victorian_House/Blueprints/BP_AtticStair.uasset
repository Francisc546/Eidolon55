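; Key-locked, interactable attic stair that toggles between open and closed with animation and sound.
; A FlipFlop and paired DoOnce nodes alternate animations and shift four boxes, delayed when opening; BeginPlay fakes a keyed interaction to start it closed.
; A looping timer syncs the Interactable component's active flag to PlayerHasKey.
; Focus drives a custom-depth outline that a retriggerable delay clears.
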(event `/Game/Victorian_House/Blueprints/BP_InteractInterface.OnInteract`
  (bind _box (`self.Box`))
  (bind _box_2 (`self.Box`))
  ;[1 1 1] Animation and Sound
  (if (`self.PlayerHasKey`)
    (`/Engine/EditorBlueprintResources/StandardMacros.FlipFlop`
      (:`A`
        (`|ExecutionSequence`
          (:`then_0`
            (`/Engine/EditorBlueprintResources/StandardMacros.DoOnce` true :!label _label
              (:`Completed`
                (`GameplayStatics.PlaySoundAtLocation` "/Game/Victorian_House/Audio/Cues/Cue_OpenAtticStair.Cue_OpenAtticStair" (0.0 0.0 0.0) (struct) 1.0 1.0 0.0 null null null null)
                (goto _label_3 :!via `Reset`))))
          (:`then_1`
            (`SkeletalMeshComponent.PlayAnimation` (`self.SM_AtticStair`) "/Game/Victorian_House/Animations/Anim_AtticStair_Close.Anim_AtticStair_Close" false)
            (`|ExecutionSequence`
              (:`then_1`
                (`/Engine/EditorBlueprintResources/StandardMacros.DoOnce` false :!label _label_2
                  (:`Completed`
                    (`SceneComponent.K2_AddRelativeRotation` _box (struct :`Roll` 60.0) false false)
                    (`SceneComponent.K2_AddRelativeRotation` (`self.Box1`) (struct :`Roll` 60.0) false false)
                    (`SceneComponent.K2_AddRelativeRotation` (`self.Box2`) (struct :`Roll` 60.0) false false)
                    (`SceneComponent.K2_AddRelativeRotation` (`self.Box3`) (struct :`Roll` 60.0) false false)
                    (`SceneComponent.K2_AddRelativeLocation` _box (0.0 0.0 160.0) false false)
                    (`SceneComponent.K2_AddRelativeLocation` (`self.Box1`) (0.0 0.0 160.0) false false)
                    (`SceneComponent.K2_AddRelativeLocation` (`self.Box2`) (0.0 0.0 160.0) false false)
                    (`SceneComponent.K2_AddRelativeLocation` (`self.Box3`) (0.0 0.0 160.0) false false)
                    (goto _label_4 :!via `Reset`))))))))
      (:`B`
        (`|ExecutionSequence`
          (:`then_0`
            (`/Engine/EditorBlueprintResources/StandardMacros.DoOnce` false :!label _label_3
              (:`Completed`
                (`GameplayStatics.PlaySoundAtLocation` "/Game/Victorian_House/Audio/Cues/Cue_CloseAtticStair.Cue_CloseAtticStair" (0.0 0.0 0.0) (struct) 1.0 1.0 0.0 null null null null)
                (goto _label :!via `Reset`))))
          (:`then_1`
            (`SkeletalMeshComponent.PlayAnimation` (`self.SM_AtticStair`) "/Game/Victorian_House/Animations/Anim_AtticStair_Open.Anim_AtticStair_Open" false)
            (`|ExecutionSequence`
              (:`then_1`
                (`KismetSystemLibrary.Delay` 2.0)
                (`/Engine/EditorBlueprintResources/StandardMacros.DoOnce` false :!label _label_4
                  (:`Completed`
                    (`SceneComponent.K2_AddRelativeRotation` _box_2 (struct :`Roll` -60.0) false false)
                    (`SceneComponent.K2_AddRelativeRotation` (`self.Box1`) (struct :`Roll` -60.0) false false)
                    (`SceneComponent.K2_AddRelativeRotation` (`self.Box2`) (struct :`Roll` -60.0) false false)
                    (`SceneComponent.K2_AddRelativeRotation` (`self.Box3`) (struct :`Roll` -60.0) false false)
                    (`SceneComponent.K2_AddRelativeLocation` _box_2 (0.0 0.0 -160.0) false false)
                    (`SceneComponent.K2_AddRelativeLocation` (`self.Box1`) (0.0 0.0 -160.0) false false)
                    (`SceneComponent.K2_AddRelativeLocation` (`self.Box2`) (0.0 0.0 -160.0) false false)
                    (`SceneComponent.K2_AddRelativeLocation` (`self.Box3`) (0.0 0.0 -160.0) false false)
                    (goto _label_2 :!via `Reset`)))))))))))

(event `/Game/Victorian_House/Blueprints/BP_InteractInterface.On Focus`
  ;[1 1 1] Outline
  (`|ExecutionSequence`
    (:`then_0`
      (if (`self.Outline on/off`)
        (`self.BeginFocus`))
      (set `self.TimeOutlineEnd` 0.1)
      (`KismetSystemLibrary.RetriggerableDelay` (`self.TimeOutlineEnd`))
      (`self.EndFocus`))))

(event `self.ReceiveBeginPlay`
  (set `self.PlayerHasKey` true)
  (`self.OnInteract`)
  (set `self.BeginPlay` false)
  (set `self.PlayerHasKey` false)
  (`KismetSystemLibrary.K2_SetTimerDelegate` (delegate `ActivateWidget`) 0.1 true)
  (`InteractableComponent.SetInteractableDataBasedOnDataTable` (`self.Interactable`) "/Game/HorrorEngine/Input/InteractionKeysUI/InteractableList.InteractableList" "AtticStairs"))

(event `ActivateWidget`
  (bind _interactable (`self.Interactable`))
  (if (`self.PlayerHasKey`)
    (`/Engine/EditorBlueprintResources/StandardMacros.DoOnce` false :!label _label_5
      (:`Completed`
        (set `InteractableComponent.bStartWithInteractionActive` true _interactable)
        (goto _label_6 :!via `Reset`)))
    (else
      (`/Engine/EditorBlueprintResources/StandardMacros.DoOnce` false :!label _label_6
        (:`Completed`
          (set `InteractableComponent.bStartWithInteractionActive` false _interactable)
          (goto _label_5 :!via `Reset`))))))

(fn `BeginFocus`
  (`PrimitiveComponent.SetRenderCustomDepth` (`self.SM_AtticStair`) true))

(fn `EndFocus`
  (`PrimitiveComponent.SetRenderCustomDepth` (`self.SM_AtticStair`) false))

(fn `UserConstructionScript`)