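; BP_Book_Inspection is a book prop that can show a focus outline, gated by the OutlineOnoff flag.
; OnFocus turns on Custom Depth rendering on MeshBook01 through BeginFocus, then starts a short retriggerable delay.
; Repeated focus calls keep resetting the delay, so EndFocus clears Custom Depth only once they stop, with no explicit unfocus event.
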(event `/Game/Victorian_House/Blueprints/BP_InteractInterface.On Focus`
  ;[1 1 1] Outline
  (`|ExecutionSequence`
    (:`then_0`
      (if (`self.Outline on/off`)
        (`self.BeginFocus`))
      (set `self.TimeOutlineEnd` 0.1)
      (`KismetSystemLibrary.RetriggerableDelay` (`self.TimeOutlineEnd`))
      (`self.EndFocus`))))

(fn `BeginFocus`
  (`PrimitiveComponent.SetRenderCustomDepth` (`self.Mesh_Book_01`) true))

(fn `EndFocus`
  (`PrimitiveComponent.SetRenderCustomDepth` (`self.Mesh_Book_01`) false))

(fn `UserConstructionScript`)