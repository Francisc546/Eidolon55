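; Victorian house wall lamp that the player can focus, highlighted through custom depth, and interact with to switch on or off.
; Interaction toggles two point lights, plays a sound at world origin, and flip-flops material emissive while destroying or respawning a BP_LightArea.
; BeginPlay always spawns that area, offset from the Lamp's relative transform, while LightOnoff sets only initial light visibility in the construction script.
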(event `self.ReceiveBeginPlay`
  (bind (_returnvalue_location _returnvalue_rotation) (`KismetMathLibrary.BreakTransform` (`SceneComponent.GetRelativeTransform` (`self.Lamp`))))
  (bind _returnvalue (`|SpawnActorFromClass` "/Game/RememberMe/BPs/Area/BP_LightArea.BP_LightArea_C" (`KismetMathLibrary.MakeTransform` (+ _returnvalue_location (0.0 -18.0 -20.0)) _returnvalue_rotation (3.0 3.0 4.0)) "Undefined" "MultiplyWithRoot" null null)))

(event `/Game/Victorian_House/Blueprints/BP_InteractInterface.OnInteract`
  (bind (_returnvalue_location _returnvalue_rotation) (`KismetMathLibrary.BreakTransform` (`SceneComponent.GetRelativeTransform` (`self.Lamp`))))
  ;[1 1 1] on/off Light
  (`SceneComponent.ToggleVisibility` (`self.PointLight2`) false)
  (`SceneComponent.ToggleVisibility` (`self.PointLight1`) false)
  (`/Engine/EditorBlueprintResources/StandardMacros.FlipFlop`
    (:`A`
      (bind _returnvalue (`PrimitiveComponent.CreateDynamicMaterialInstance` (`self.Lamp`) 2 "/Game/Victorian_House/Materials/Instance/Tiling/Inst_Plastic_Glossy_02.Inst_Plastic_Glossy_02" "None"))
      (set `self.Dynamic material` _returnvalue)
      (`MaterialInstanceDynamic.SetScalarParameterValue` (`self.Dynamic material`) "PowerEmissive" 0.0)
      (`self.K2_DestroyActor` (stale _returnvalue_3))
      (`self.K2_DestroyActor` (stale `self.ReceiveBeginPlay` _returnvalue)))
    (:`B`
      (bind _returnvalue_2 (`PrimitiveComponent.CreateDynamicMaterialInstance` (`self.Lamp`) 2 "/Game/Victorian_House/Materials/Instance/Tiling/Inst_Plastic_Glossy_02.Inst_Plastic_Glossy_02" "None"))
      (set `self.Dynamic material` _returnvalue_2)
      (`MaterialInstanceDynamic.SetScalarParameterValue` (`self.Dynamic material`) "PowerEmissive" 5.0)
      (bind _returnvalue_3 (`|SpawnActorFromClass` "/Game/RememberMe/BPs/Area/BP_LightArea.BP_LightArea_C" (`KismetMathLibrary.MakeTransform` (+ _returnvalue_location (0.0 -18.0 -20.0)) _returnvalue_rotation (3.0 3.0 4.0)) "Undefined" "MultiplyWithRoot" null null))))
  (`GameplayStatics.PlaySoundAtLocation` "/Game/Victorian_House/Audio/Cues/Cue_Light.Cue_Light" (0.0 0.0 0.0) (struct) 1.0 1.0 0.0 null null null null))

(fn `BeginFocus`
  (`PrimitiveComponent.SetRenderCustomDepth` (`self.Lamp`) true))

(fn `EndFocus`
  (`PrimitiveComponent.SetRenderCustomDepth` (`self.Lamp`) false))

(fn `UserConstructionScript`
  ;[1 1 1] on/off Light
  (`SceneComponent.SetVisibility` (`self.PointLight2`) (`self.Light on/off `) false)
  (`SceneComponent.SetVisibility` (`self.PointLight1`) (`self.Light on/off `) false))