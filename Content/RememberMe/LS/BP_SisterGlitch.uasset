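; BP_SisterGlitch is a one-shot trigger that plays the sister glitch cutscene when the player enters its box.
; It locks player input, plays LS_SisterGlitch, shows the Emily_Hey video fullscreen through WBP_IntroVideo, then plays LS_SisterGlitchPart2.
; Delays based on sequence and media lengths chain the stages.
; Afterwards it restores game input, clears the player's DisableDot flag and destroys itself.
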(event `self.Box.OnComponentBeginOverlap`
  (params (OverlappedComponent :type "PrimitiveComponent Object Reference") (OtherActor :type "Actor Object Reference") (OtherComp :type "PrimitiveComponent Object Reference") (OtherBodyIndex :type Integer) (bFromSweep :type Boolean) (SweepResult :type "HitResult Structure (by ref)"))
  (bind _returnvalue (`GameplayStatics.GetPlayerController` 0))
  (bind _returnvalue_2 (`GameplayStatics.GetPlayerController` 0))
  (bind _mediaplayer (`self.MediaPlayer`))
  (if (== OtherActor (`GameplayStatics.GetPlayerPawn` 0))
    (bind _asmaster (`/Game/HorrorEngine/Blueprints/Core/HE_Functions.GetPlayer`))
    (`self.DisableInput` _asmaster _returnvalue)
    (`WidgetBlueprintLibrary.SetInputMode_UIOnlyEx` _returnvalue null "LockAlways" true)
    (bind (_outactor _returnvalue_3) (`LevelSequencePlayer.CreateLevelSequencePlayer` "/Game/RememberMe/LS/LS_SisterGlitch.LS_SisterGlitch"))
    (`MovieSceneSequencePlayer.Play` (`LevelSequenceActor.SequencePlayer` _outactor))
    (`KismetSystemLibrary.Delay` (`TimeManagementBlueprintLibrary.Conv_QualifiedFrameTimeToSeconds` (`MovieSceneSequencePlayer.GetEndTime` _returnvalue_3)))
    (`AddComponent|NODE_AddMediaSoundComponent-0`)
    (`MediaPlayer.OpenSource` _mediaplayer "/Game/Movies/Emily_Hey.Emily_Hey")
    (bind _returnvalue_4 (`|CreateWidget` "/Game/RememberMe/Widgets/VIdeoPlayback/WBP_IntroVideo.WBP_IntroVideo_C" null _mediaplayer "/Game/Movies/Emily_Hey.Emily_Hey"))
    (`UserWidget.AddToViewport` _returnvalue_4 0)
    (`Image.SetBrush` (`/Game/RememberMe/Widgets/VIdeoPlayback/WBP_IntroVideo.VideoSuccess` _returnvalue_4) (make `SlateBrush` "Image" "NoTile" "NoMirror" (struct :`X` 32.0 :`Y` 32.0) (struct) (struct :`SpecifiedColor` (struct :`R` 1.0 :`G` 1.0 :`B` 1.0 :`A` 1.0) :`ColorUseRule` "UseColor_Specified") (struct :`CornerRadii` (struct) :`Color` (struct :`SpecifiedColor` (struct) :`ColorUseRule` "UseColor_Specified") :`RoundingType` "HalfHeightRadius") "/Game/Movies/EmilyHey_MediaTexture_Mat.EmilyHey_MediaTexture_Mat"))
    (`MediaPlayer.Play` _mediaplayer)
    (`KismetSystemLibrary.Delay` 0.2)
    (`/Game/RememberMe/Widgets/VIdeoPlayback/WBP_IntroVideo.DecreaseOpacityPrompt` _returnvalue_4)
    (`KismetSystemLibrary.Delay` (`KismetMathLibrary.GetTotalSeconds` (`MediaPlayer.GetDuration` _mediaplayer)))
    (bind _outactor_2 (`LevelSequencePlayer.CreateLevelSequencePlayer` "/Game/RememberMe/LS/LS_SisterGlitchPart2.LS_SisterGlitchPart2"))
    (`Widget.RemoveFromParent` _returnvalue_4)
    (bind _sequenceplayer (`LevelSequenceActor.SequencePlayer` _outactor_2))
    (`MovieSceneSequencePlayer.Play` _sequenceplayer)
    (`KismetSystemLibrary.Delay` (`TimeManagementBlueprintLibrary.Conv_QualifiedFrameTimeToSeconds` (`MovieSceneSequencePlayer.GetEndTime` _sequenceplayer)))
    (bind _asmaster_2 (`/Game/HorrorEngine/Blueprints/Core/HE_Functions.GetPlayer`))
    (`self.EnableInput` _asmaster_2 _returnvalue_2)
    (`WidgetBlueprintLibrary.SetInputMode_GameOnly` _returnvalue_2)
    (bind _asmaster_3 (`/Game/HorrorEngine/Blueprints/Core/HE_Functions.GetPlayer`))
    (set `/Game/HorrorEngine/Blueprints/Player/HorrorEngine.DisableDot` false _asmaster_3)
    (`self.K2_DestroyActor`)))

(fn `UserConstructionScript`)