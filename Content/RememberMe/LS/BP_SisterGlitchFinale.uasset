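; Trigger actor that plays a subtitle and then brings in the house manager, named for the sister glitch finale.
; When the player pawn overlaps its Box, it creates a Subtitle_WB widget and shows TomySubtitle from the first line.
; After a delay taken from that first entry's duration, it spawns BP_HouseManager and destroys itself.
; A StartRetry event shares the same player-checked path.
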(event `StartRetry`
  (bind _tomysubtitle (`self.TomySubtitle`))
  (if (== (stale `self.Box.OnComponentBeginOverlap` OtherActor) (`GameplayStatics.GetPlayerPawn` 0)) :!label _label
    (bind _subtitlewidget (`self.CreateSubtitleWidget`))
    (`/Game/HorrorEngine/Blueprints/Widgets/MainHUD/Subtitle_WB.SubtitleText` _subtitlewidget _tomysubtitle 0)
    (`KismetSystemLibrary.Delay` (`.ModifyDuration+or-Sec_46_08FC403D464A20C6CBF55A82BF774C1F` (break `/Game/HorrorEngine/Blueprints/Structures/HorrorEvent/HE_Subtitle` (`|GetArrayItem` _tomysubtitle))))
    (`|SpawnActorFromClass` "/Game/RememberMe/BPs/BP_HouseManager.BP_HouseManager_C" (`KismetMathLibrary.MakeTransform` (0.0 0.0 0.0)) "Undefined" "MultiplyWithRoot" null null)
    (`self.K2_DestroyActor`)))

(event `self.Box.OnComponentBeginOverlap`
  (params (OverlappedComponent :type "PrimitiveComponent Object Reference") (OtherActor :type "Actor Object Reference") (OtherComp :type "PrimitiveComponent Object Reference") (OtherBodyIndex :type Integer) (bFromSweep :type Boolean) (SweepResult :type "HitResult Structure (by ref)"))
  (goto _label))

(fn `CreateSubtitleWidget`
  (returns (SubtitleWidget :type "/Game/HorrorEngine/Blueprints/Widgets/MainHUD/Subtitle_WB Object Reference"))
  (bind _returnvalue (`|CreateWidget` "/Game/HorrorEngine/Blueprints/Widgets/MainHUD/Subtitle_WB.Subtitle_WB_C"))
  (`UserWidget.AddToViewport` _returnvalue 0)
  (return _returnvalue))

(fn `UserConstructionScript`)