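; End-game Blueprint that shows the finishing video, then hands the player over to the end screen.
; On BeginPlay, after a short delay, it adds a media sound component and reuses WBP_IntroVideo with the M_End brush, passing in the media player and source.
; It waits out the player's reported duration, then swaps to WBP_EndGameEidolon with UI-only input and a visible cursor.
; A subtitle-widget helper is defined but not called here.
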(event `self.ReceiveBeginPlay`
  (bind _returnvalue (`GameplayStatics.GetPlayerController` 0))
  (bind _mplay_1 (`self.MPlay 1`))
  (`KismetSystemLibrary.Delay` 4.2)
  (`AddComponent|NODE_AddMediaSoundComponent-0`)
  (bind _returnvalue_2 (`|CreateWidget` "/Game/RememberMe/Widgets/VIdeoPlayback/WBP_IntroVideo.WBP_IntroVideo_C" null _mplay_1 (`self.Media Source`)))
  (`Image.SetBrush` (`/Game/RememberMe/Widgets/VIdeoPlayback/WBP_IntroVideo.VideoSuccess` _returnvalue_2) (make `SlateBrush` "Image" "NoTile" "NoMirror" (struct :`X` 32.0 :`Y` 32.0) (struct) (struct :`SpecifiedColor` (struct :`R` 1.0 :`G` 1.0 :`B` 1.0 :`A` 1.0) :`ColorUseRule` "UseColor_Specified") (struct :`CornerRadii` (struct) :`Color` (struct :`SpecifiedColor` (struct) :`ColorUseRule` "UseColor_Specified") :`RoundingType` "HalfHeightRadius") "/Game/Movies/M_End.M_End"))
  (`UserWidget.AddToViewport` _returnvalue_2 0)
  (`KismetSystemLibrary.Delay` 0.1)
  (`KismetSystemLibrary.Delay` (`KismetMathLibrary.GetTotalSeconds` (`MediaPlayer.GetDuration` _mplay_1)))
  (`WidgetBlueprintLibrary.SetInputMode_UIOnlyEx` _returnvalue null)
  (`Widget.RemoveFromParent` _returnvalue_2)
  (set `PlayerController.bShowMouseCursor` true _returnvalue)
  (bind _returnvalue_3 (`|CreateWidget` "/Game/RememberMe/Widgets/WBP_EndGameEidolon.WBP_EndGameEidolon_C"))
  (`UserWidget.AddToViewport` _returnvalue_3 0))

(fn `CreateSubtitleWidget`
  (returns (SubtitleW :type "/Game/HorrorEngine/Blueprints/Widgets/MainHUD/Subtitle_WB Object Reference"))
  (bind _returnvalue (`|CreateWidget` "/Game/HorrorEngine/Blueprints/Widgets/MainHUD/Subtitle_WB.Subtitle_WB_C"))
  (`UserWidget.AddToViewport` _returnvalue 0)
  (return _returnvalue))

(fn `UserConstructionScript`)