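; Level manager for the white room sequence, driving narrative subtitles and reacting to three VHS flags.
; A looping timer polls the flags; once all are set, it plays chained subtitles timed by delays, turns on the middle TV with a Mnemosyne channel, then shows narrative options.
; BringButtonUp raises the tagged button by timeline, but the timer's route to it is unreachable because the counter is forced to 3.
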(event `BringButtonUp`
  (bind _outactors (`GameplayStatics.GetAllActorsOfClassWithTag` "/Game/HorrorEngine/Blueprints/Assets/Interactables/RoundButton.RoundButton_C" "WhiteRoom"))
  (`/Game/HorrorEngine/Blueprints/Core/HE_Functions.Notice` "A" "button" "is rising from the floor")
  (bind (_direction _zheight) (`Timeline|Timeline` :!via `PlayFromStart`)
    (:`Update`
      (bind _rootcomponent (`Actor.RootComponent` (`|GetArrayItem` _outactors)))
      (bind (_returnvalue_x _returnvalue_y) (`KismetMathLibrary.BreakVector` (`SceneComponent.K2_GetComponentLocation` _rootcomponent)))
      (`SceneComponent.K2_SetWorldLocation` _rootcomponent (`KismetMathLibrary.MakeVector` _returnvalue_x _returnvalue_y _zheight) false false))))

(event `self.ReceiveBeginPlay`
  (bind _doyouwho (`self.DoYouWho`))
  ; Create new widget everytime
  (bind _subtitlew (`self.CreateSubtitleWidget`))
  (`/Game/HorrorEngine/Blueprints/Widgets/MainHUD/Subtitle_WB.SubtitleText` _subtitlew _doyouwho 0)
  (`KismetSystemLibrary.Delay` (* (`.ModifyDuration+or-Sec_46_08FC403D464A20C6CBF55A82BF774C1F` (break `/Game/HorrorEngine/Blueprints/Structures/HorrorEvent/HE_Subtitle` (`|GetArrayItem` _doyouwho))) 1.1))
  (bind _subtitlew_2 (`self.CreateSubtitleWidget`))
  (`/Game/HorrorEngine/Blueprints/Widgets/MainHUD/Subtitle_WB.SubtitleText` _subtitlew_2 (`self.Subtitle2`) 0)
  (`KismetSystemLibrary.K2_SetTimerDelegate` (delegate `CheckCounter`) 0.1 true))

(event `CheckCounter`
  (bind _doyouwho (`self.DoYouWho`))
  (bind _subtitle3 (`self.Subtitle3`))
  (bind _subtitle4 (`self.Subtitle4`))
  (bind _subtitle5 (`self.Subtitle5`))
  (bind _vhscounter (`self.VHSCounter`))
  (if (and (`self.VHS2`) (`self.VHS3`) (`self.VHS1`))
    (set `self.VHSCounter` 3)
    (if (>= _vhscounter 3)
      (if (>= _vhscounter 5)
        (`/Engine/EditorBlueprintResources/StandardMacros.DoOnce` false
          (:`Completed`
            (`self.BringButtonUp`)))
        (else
          (`/Engine/EditorBlueprintResources/StandardMacros.DoOnce` false
            (:`Completed`
              (bind _subtitlew (`self.CreateSubtitleWidget`))
              (`/Game/HorrorEngine/Blueprints/Widgets/MainHUD/Subtitle_WB.SubtitleText` _subtitlew _subtitle3 0)
              (`KismetSystemLibrary.Delay` (* (`.ModifyDuration+or-Sec_46_08FC403D464A20C6CBF55A82BF774C1F` (break `/Game/HorrorEngine/Blueprints/Structures/HorrorEvent/HE_Subtitle` (`|GetArrayItem` _subtitle3))) 1.1))
              (bind _subtitlew_2 (`self.CreateSubtitleWidget`))
              (`/Game/HorrorEngine/Blueprints/Widgets/MainHUD/Subtitle_WB.SubtitleText` _subtitlew_2 _doyouwho 0)
              (`KismetSystemLibrary.Delay` (* (`.ModifyDuration+or-Sec_46_08FC403D464A20C6CBF55A82BF774C1F` (break `/Game/HorrorEngine/Blueprints/Structures/HorrorEvent/HE_Subtitle` (`|GetArrayItem` _doyouwho))) 1.1))
              (bind _subtitlew_3 (`self.CreateSubtitleWidget`))
              (`/Game/HorrorEngine/Blueprints/Widgets/MainHUD/Subtitle_WB.SubtitleText` _subtitlew_3 _subtitle4 0)
              (`KismetSystemLibrary.Delay` (* (`.ModifyDuration+or-Sec_46_08FC403D464A20C6CBF55A82BF774C1F` (break `/Game/HorrorEngine/Blueprints/Structures/HorrorEvent/HE_Subtitle` (`|GetArrayItem` _subtitle4))) 1.1))
              (bind _subtitlew_4 (`self.CreateSubtitleWidget`))
              (`/Game/HorrorEngine/Blueprints/Widgets/MainHUD/Subtitle_WB.SubtitleText` _subtitlew_4 _subtitle5 0)
              ; Place Player in position and rotation to see all 3 screens
              (bind _outactors (`GameplayStatics.GetAllActorsOfClassWithTag` "/Game/HorrorEngine/Blueprints/Assets/Interactables/TV.TV_C" "Middle"))
              (bind _output (`|GetArrayItem` _outactors))
              (`KismetArrayLibrary.Array_Add` (`/Game/HorrorEngine/Blueprints/Assets/Interactables/TV.AddChannels` _output) "/Game/Movies/Mnemosyne.Mnemosyne")
              (set `/Game/HorrorEngine/Blueprints/Assets/Interactables/TV.Looping` true _output)
              (`/Game/HorrorEngine/Blueprints/Core/Use.Open/On` _output false)
              (set `/Game/HorrorEngine/Blueprints/Assets/Interactables/TV.On / Off` true _output)
              (`KismetSystemLibrary.Delay` (* (`.ModifyDuration+or-Sec_46_08FC403D464A20C6CBF55A82BF774C1F` (break `/Game/HorrorEngine/Blueprints/Structures/HorrorEvent/HE_Subtitle` (`|GetArrayItem` _subtitle5))) 1.1))
              (bind _returnvalue (`|CreateWidget` "/Game/RememberMe/Widgets/WBP_NarrativeOptions.WBP_NarrativeOptions_C"))
              (`UserWidget.AddToViewport` _returnvalue 0))))))))

(fn `CreateSubtitleWidget`
  (returns (SubtitleW :type "/Game/HorrorEngine/Blueprints/Widgets/MainHUD/Subtitle_WB Object Reference"))
  (bind _returnvalue (`|CreateWidget` "/Game/HorrorEngine/Blueprints/Widgets/MainHUD/Subtitle_WB.Subtitle_WB_C"))
  (`UserWidget.AddToViewport` _returnvalue 0)
  (return _returnvalue))

(fn `UserConstructionScript`)