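; BP_LightArea is a trigger volume that reveals hidden-message papers while the player is inside it.
; When the player pawn begins overlapping its Box, it clears the Hidden flag on every HiddenMessagePaper actor in the level and refreshes each one's texture.
; When the player pawn leaves, it sets the flag again and refreshes them, so the effect is global rather than limited to papers inside the area.
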(event `self.Box.OnComponentBeginOverlap`
  (params (OverlappedComponent :type "PrimitiveComponent Object Reference") (OtherActor :type "Actor Object Reference") (OtherComp :type "PrimitiveComponent Object Reference") (OtherBodyIndex :type Integer) (bFromSweep :type Boolean) (SweepResult :type "HitResult Structure (by ref)"))
  (if (== OtherActor (`GameplayStatics.GetPlayerPawn` 0))
    (bind _outactors (`GameplayStatics.GetAllActorsOfClass` "/Game/HorrorEngine/Blueprints/UseableAssets/Inventory/HiddenMessagePaper.HiddenMessagePaper_C"))
    (for _array_element _outactors
      (set `/Game/HorrorEngine/Blueprints/UseableAssets/Inventory/HiddenMessagePaper.Hidden` false _array_element)
      (`/Game/HorrorEngine/Blueprints/UseableAssets/Inventory/HiddenMessagePaper.RefreshTexture` _array_element))))

(event `self.Box.OnComponentEndOverlap`
  (params (OverlappedComponent :type "PrimitiveComponent Object Reference") (OtherActor :type "Actor Object Reference") (OtherComp :type "PrimitiveComponent Object Reference") (OtherBodyIndex :type Integer))
  (if (== OtherActor (`GameplayStatics.GetPlayerPawn` 0))
    (bind _outactors (`GameplayStatics.GetAllActorsOfClass` "/Game/HorrorEngine/Blueprints/UseableAssets/Inventory/HiddenMessagePaper.HiddenMessagePaper_C"))
    (for _array_element _outactors
      (set `/Game/HorrorEngine/Blueprints/UseableAssets/Inventory/HiddenMessagePaper.Hidden` true _array_element)
      (`/Game/HorrorEngine/Blueprints/UseableAssets/Inventory/HiddenMessagePaper.RefreshTexture` _array_element))))

(fn `UserConstructionScript`)