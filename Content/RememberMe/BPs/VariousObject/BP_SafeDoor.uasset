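; Safe door actor that, once unlocked, swings open and closed on alternating interactions through a timeline-driven yaw rotation.
; The first open and first close each play a sound and set Takeable on the "Safe"-tagged InspectableObjects actor, behind never-reset DoOnce gates.
; Focus shows a custom-depth outline that a retriggerable delay clears.
; The construction script attaches AttachedActors to the door mesh.
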(event `/Game/Victorian_House/Blueprints/BP_InteractInterface.OnInteract`
  ;[1 1 1] Open Door
  (if (`self.Unlocked`)
    (`/Engine/EditorBlueprintResources/StandardMacros.FlipFlop`
      (:`A`
        (`|ExecutionSequence`
          (:`then_0`
            (`/Engine/EditorBlueprintResources/StandardMacros.DoOnce` false
              (:`Completed`
                (`GameplayStatics.PlaySoundAtLocation` "/Game/Victorian_House/Audio/Cues/Cue_OpenDoor_02.Cue_OpenDoor_02" (0.0 0.0 0.0) (struct) 1.0 1.0 0.0 null null null null)
                (bind _outactors (`GameplayStatics.GetAllActorsOfClassWithTag` "/Game/RememberMe/BPs/VariousObject/InspectableObjects.InspectableObjects_C" "Safe"))
                (set `/Game/HorrorEngine/Blueprints/Core/Inspectable.Takeable` true (`|GetArrayItem` _outactors)))))
          (:`then_1`
            (bind (_direction _newtrack_0) (`Timeline|Timeline_0` :!label _label)
              (:`Update`
                (`SceneComponent.K2_SetRelativeRotation` (`self.Mesh_Cupboard_01_Door_02`) (`KismetMathLibrary.MakeRotator` 0.0 0.0 _newtrack_0) false false))))))
      (:`B`
        (`|ExecutionSequence`
          (:`then_0`
            (goto _label :!via `Reverse`))
          (:`then_1`
            (`/Engine/EditorBlueprintResources/StandardMacros.DoOnce` false
              (:`Completed`
                (`GameplayStatics.PlaySoundAtLocation` "/Game/Victorian_House/Audio/Wavs/S_CloseDoor_02.S_CloseDoor_02" (0.0 0.0 0.0) (struct) 1.0 1.0 0.0 null null null null)
                (bind _outactors_2 (`GameplayStatics.GetAllActorsOfClassWithTag` "/Game/RememberMe/BPs/VariousObject/InspectableObjects.InspectableObjects_C" "Safe"))
                (set `/Game/HorrorEngine/Blueprints/Core/Inspectable.Takeable` false (`|GetArrayItem` _outactors_2))))))))))

(event `/Game/Victorian_House/Blueprints/BP_InteractInterface.On Focus`
  ;[1 1 1] Outline
  (`|ExecutionSequence`
    (:`then_0`
      (if (`self.Outline on/off`)
        (`self.BeginFocus`))
      (set `self.TimeOutlineEnd` 0.1)
      (`KismetSystemLibrary.RetriggerableDelay` (`self.TimeOutlineEnd`))
      (`self.EndFocus`))))

(fn `BeginFocus`
  (`PrimitiveComponent.SetRenderCustomDepth` (`self.Mesh_Cupboard_01_Door_02`) true))

(fn `EndFocus`
  (`PrimitiveComponent.SetRenderCustomDepth` (`self.Mesh_Cupboard_01_Door_02`) false))

(fn `UserConstructionScript`
  (for _array_element (`self.AttachedActors`)
    (`self.K2_AttachToComponent` _array_element (`self.Mesh_Cupboard_01_Door_02`) "None" "KeepWorld" "KeepWorld" "KeepWorld" true)))