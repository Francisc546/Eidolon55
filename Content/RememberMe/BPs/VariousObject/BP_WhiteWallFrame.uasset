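; Interactive wall frame puzzle where the player previews five memory clips and puts them in the correct order.
; Use toggles a camera blend to the frame, locking movement and look and showing WBP_ViewClips.
; A highlight selects buttons whose material names pick the clip to play, and reordering swaps materials between neighbours, wrapping around.
; Confirming compares material names to SolutionArray; success unloads data layers, spawns BP_FinishGame, shows a subtitle and destroys house managers.
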(event `BackToFrame`
  (bind _returnvalue (`GameplayStatics.GetPlayerController` 0))
  ;[1 1 1] ZoomIn
  (`PlayerController.SetViewTargetWithBlend` _returnvalue self 1.0 "VTBlend_Linear" 0.0 true :!label _label)
  (set `CharacterMovementComponent.MaxWalkSpeed` 0.0 (`Character.CharacterMovement` (`GameplayStatics.GetPlayerCharacter` 0)))
  (`PlayerController.SetDeprecatedInputPitchScale` _returnvalue 0.0)
  (`PlayerController.SetDeprecatedInputYawScale` _returnvalue 0.0)
  (bind _returnvalue_2 (`|CreateWidget` "/Game/RememberMe/Widgets/WBP_ViewClips.WBP_ViewClips_C" null self))
  (`UserWidget.AddToViewport` _returnvalue_2 0))

(event `self.Use`
  (params (HorrorEvent :type Boolean))
  (bind _returnvalue (`GameplayStatics.GetPlayerController` 0))
  (bind _selectedbutton (`self.SelectedButton`))
  (if (not (`self.Disabled`))
    (`/Engine/EditorBlueprintResources/StandardMacros.FlipFlop`
      (:`A`
        ;[1 1 1] ZoomIn
        (`SceneComponent.SetVisibility` _selectedbutton true true)
        (goto _label))
      (:`B`
        ;[1 1 1] ZoomOut
        (`SceneComponent.SetVisibility` _selectedbutton false true)
        (`PlayerController.SetViewTargetWithBlend` _returnvalue (`GameplayStatics.GetPlayerCharacter` 0) 1.0 "VTBlend_Linear" 0.0 true :!label _label_2)
        (set `CharacterMovementComponent.MaxWalkSpeed` 150.0 (`Character.CharacterMovement` (`GameplayStatics.GetPlayerCharacter` 0)))
        (`PlayerController.SetDeprecatedInputPitchScale` _returnvalue -2.0)
        (`PlayerController.SetDeprecatedInputYawScale` _returnvalue 2.0)
        (`Widget.RemoveFromParent` (stale `BackToFrame` _returnvalue_2))))))

(event `ExitFrame`
  (goto _label_2))

(event `self.ReceiveBeginPlay`
  (`PrimitiveComponent.SetMaterial` (`self.Button1`) 0 (`self.Material1`))
  (`PrimitiveComponent.SetMaterial` (`self.Button2`) 0 (`self.Material2`))
  (`PrimitiveComponent.SetMaterial` (`self.Button3`) 0 (`self.Material3`))
  (`PrimitiveComponent.SetMaterial` (`self.Button4`) 0 (`self.Material4`))
  (`PrimitiveComponent.SetMaterial` (`self.Button5`) 0 (`self.Material5`)))

(event `Play`
  (bind (_mediasource _mplay) (`self.SetMediaSource`))
  (bind _returnvalue (`|CreateWidget` "/Game/RememberMe/Widgets/VIdeoPlayback/WBP_PlaybackVideo.WBP_PlaybackVideo_C" null _mediasource (`self.CurrentValue`)))
  (`UserWidget.AddToViewport` _returnvalue 0))

(event `Reorder`
  (bind _currentvalue (`self.CurrentValue`))
  (set `self.CurrentValueReorder` _currentvalue)
  (switch `int` _currentvalue
    (:`1`
      (set `self.CurrentMaterial` (`PrimitiveComponent.GetMaterial` (`self.Button1`) 0)))
    (:`2`
      (set `self.CurrentMaterial` (`PrimitiveComponent.GetMaterial` (`self.Button2`) 0)))
    (:`3`
      (set `self.CurrentMaterial` (`PrimitiveComponent.GetMaterial` (`self.Button3`) 0)))
    (:`4`
      (set `self.CurrentMaterial` (`PrimitiveComponent.GetMaterial` (`self.Button4`) 0)))
    (:`5`
      (set `self.CurrentMaterial` (`PrimitiveComponent.GetMaterial` (`self.Button5`) 0)))))

(event `ReorderRight`
  (bind _buttonn (`self.GetSelectedButton`))
  (`self.ChangeButtonsMaterialsRight` _buttonn))

(event `MoveRight`
  (switch `int` (`self.CurrentValue`)
    (:`1`
      (set `self.CurrentValue` 2)
      (`SceneComponent.K2_SetWorldLocation` (`self.SelectedButton`) (`SceneComponent.K2_GetComponentLocation` (`self.Button2`)) false false))
    (:`2`
      (set `self.CurrentValue` 3)
      (`SceneComponent.K2_SetWorldLocation` (`self.SelectedButton`) (`SceneComponent.K2_GetComponentLocation` (`self.Button3`)) false false))
    (:`3`
      (set `self.CurrentValue` 4)
      (`SceneComponent.K2_SetWorldLocation` (`self.SelectedButton`) (`SceneComponent.K2_GetComponentLocation` (`self.Button4`)) false false))
    (:`4`
      (set `self.CurrentValue` 5)
      (`SceneComponent.K2_SetWorldLocation` (`self.SelectedButton`) (`SceneComponent.K2_GetComponentLocation` (`self.Button5`)) false false))
    (:`5`
      (set `self.CurrentValue` 1)
      (`SceneComponent.K2_SetWorldLocation` (`self.SelectedButton`) (`SceneComponent.K2_GetComponentLocation` (`self.Button1`)) false false))))

(event `MoveLeft`
  (switch `int` (`self.CurrentValue`)
    (:`1`
      (set `self.CurrentValue` 5)
      (`SceneComponent.K2_SetWorldLocation` (`self.SelectedButton`) (`SceneComponent.K2_GetComponentLocation` (`self.Button5`)) false false))
    (:`2`
      (set `self.CurrentValue` 1)
      (`SceneComponent.K2_SetWorldLocation` (`self.SelectedButton`) (`SceneComponent.K2_GetComponentLocation` (`self.Button1`)) false false))
    (:`3`
      (set `self.CurrentValue` 2)
      (`SceneComponent.K2_SetWorldLocation` (`self.SelectedButton`) (`SceneComponent.K2_GetComponentLocation` (`self.Button2`)) false false))
    (:`4`
      (set `self.CurrentValue` 3)
      (`SceneComponent.K2_SetWorldLocation` (`self.SelectedButton`) (`SceneComponent.K2_GetComponentLocation` (`self.Button3`)) false false))
    (:`5`
      (set `self.CurrentValue` 4)
      (`SceneComponent.K2_SetWorldLocation` (`self.SelectedButton`) (`SceneComponent.K2_GetComponentLocation` (`self.Button4`)) false false))))

(event `ReorderLeft`
  (bind _buttonn (`self.GetSelectedButton`))
  (`self.ChangeButtonsMaterialsLeft` _buttonn))

(event `ConfirmOrder`
  (bind _returnvalue (`self.VerifyCombination`))
  (if _returnvalue
    (`DataLayerSubsystem.SetDataLayerRuntimeState` (subsystem `DataLayerSubsystem`) (`self.MeetingRoom`) "Unloaded" false)
    (`DataLayerSubsystem.SetDataLayerRuntimeState` (subsystem `DataLayerSubsystem`) (`self.Mansion`) "Unloaded" false)
    (`|SpawnActorFromClass` "/Game/RememberMe/BPs/BP_FinishGame.BP_FinishGame_C" (`KismetMathLibrary.MakeTransform` (0.0 0.0 0.0)) "Undefined" "MultiplyWithRoot" null null)
    (`DataLayerSubsystem.SetDataLayerRuntimeState` (subsystem `DataLayerSubsystem`) (`self.ExitWRRoom`) "Unloaded" false)
    (`self.ExitFrame`)
    (bind _returnvalue_2 (`|CreateWidget` "/Game/HorrorEngine/Blueprints/Widgets/MainHUD/Subtitle_WB.Subtitle_WB_C"))
    (`UserWidget.AddToViewport` _returnvalue_2 0)
    (`/Game/HorrorEngine/Blueprints/Widgets/MainHUD/Subtitle_WB.SubtitleText` _returnvalue_2 (`|MakeArray` (make `/Game/HorrorEngine/Blueprints/Structures/HorrorEvent/HE_Subtitle` "Denial complete. Prepare for the next phase." "/Game/RememberMe/Dialogue/AI/DenialComplete.DenialComplete" false (struct) 4.44) :!type "/Game/HorrorEngine/Blueprints/Structures/HorrorEvent/HE_Subtitle Structure") 0)
    (bind _outactors (`GameplayStatics.GetAllActorsOfClass` "/Game/RememberMe/BPs/BP_HouseManager.BP_HouseManager_C"))
    (for _array_element _outactors
      (`self.K2_DestroyActor` _array_element))
    (else
      (`/Game/HorrorEngine/Blueprints/Core/HE_Functions.Notice` "The order is" "wrong" "!"))))

(fn `AlternativeOrderingOption`
  (bind _button5 (`self.Button5`))
  (bind _button4 (`self.Button4`))
  (bind _button3 (`self.Button3`))
  (bind _button2 (`self.Button2`))
  (bind _button1 (`self.Button1`))
  (`|ExecutionSequence`
    (:`then_0`
      (switch `int` (`self.CurrentValue`)
        (:`1`
          (set `self.SwapMaterial` (`PrimitiveComponent.GetMaterial` _button1 0))
          (`PrimitiveComponent.SetMaterial` _button1 0 (`self.CurrentMaterial`)))
        (:`2`
          (set `self.SwapMaterial` (`PrimitiveComponent.GetMaterial` _button2 0))
          (`PrimitiveComponent.SetMaterial` _button2 0 (`self.CurrentMaterial`)))
        (:`3`
          (set `self.SwapMaterial` (`PrimitiveComponent.GetMaterial` _button3 0))
          (`PrimitiveComponent.SetMaterial` _button3 0 (`self.CurrentMaterial`)))
        (:`4`
          (set `self.SwapMaterial` (`PrimitiveComponent.GetMaterial` _button4 0))
          (`PrimitiveComponent.SetMaterial` _button4 0 (`self.CurrentMaterial`)))
        (:`5`
          (set `self.SwapMaterial` (`PrimitiveComponent.GetMaterial` _button5 0))
          (`PrimitiveComponent.SetMaterial` _button5 0 (`self.CurrentMaterial`)))))
    (:`then_1`
      (switch `int` (`self.CurrentValueReorder`)
        (:`1`
          (`PrimitiveComponent.SetMaterial` (`self.Button1`) 0 (`self.SwapMaterial`)))
        (:`2`
          (`PrimitiveComponent.SetMaterial` (`self.Button2`) 0 (`self.SwapMaterial`)))
        (:`3`
          (`PrimitiveComponent.SetMaterial` (`self.Button3`) 0 (`self.SwapMaterial`)))
        (:`4`
          (`PrimitiveComponent.SetMaterial` (`self.Button4`) 0 (`self.SwapMaterial`)))
        (:`5`
          (`PrimitiveComponent.SetMaterial` (`self.Button5`) 0 (`self.SwapMaterial`)))))))

(fn `ChangeButtonsMaterialsLeft`
  (params (`Button N` :type "PrimitiveComponent Object Reference"))
  (bind _button5 (`self.Button5`))
  (bind _button1 (`self.Button1`))
  (bind _button2 (`self.Button2`))
  (bind _button3 (`self.Button3`))
  (bind _button4 (`self.Button4`))
  (switch `int` (`self.CurrentValueReorder`)
    (:`1`
      (`SceneComponent.K2_SetWorldLocation` (`self.SelectedButton`) (`SceneComponent.K2_GetComponentLocation` _button5) false false)
      (`PrimitiveComponent.SetMaterial` `Button N` 0 (`PrimitiveComponent.GetMaterial` _button5 0))
      (`PrimitiveComponent.SetMaterial` _button5 0 (`self.CurrentMaterial`))
      (set `self.CurrentValue` 5)
      (set `self.CurrentValueReorder` 5))
    (:`2`
      (`SceneComponent.K2_SetWorldLocation` (`self.SelectedButton`) (`SceneComponent.K2_GetComponentLocation` _button1) false false)
      (`PrimitiveComponent.SetMaterial` `Button N` 0 (`PrimitiveComponent.GetMaterial` _button1 0))
      (`PrimitiveComponent.SetMaterial` _button1 0 (`self.CurrentMaterial`))
      (set `self.CurrentValue` 1)
      (set `self.CurrentValueReorder` 1))
    (:`3`
      (`SceneComponent.K2_SetWorldLocation` (`self.SelectedButton`) (`SceneComponent.K2_GetComponentLocation` _button2) false false)
      (`PrimitiveComponent.SetMaterial` `Button N` 0 (`PrimitiveComponent.GetMaterial` _button2 0))
      (`PrimitiveComponent.SetMaterial` _button2 0 (`self.CurrentMaterial`))
      (set `self.CurrentValue` 2)
      (set `self.CurrentValueReorder` 2))
    (:`4`
      (`SceneComponent.K2_SetWorldLocation` (`self.SelectedButton`) (`SceneComponent.K2_GetComponentLocation` _button3) false false)
      (`PrimitiveComponent.SetMaterial` `Button N` 0 (`PrimitiveComponent.GetMaterial` _button3 0))
      (`PrimitiveComponent.SetMaterial` _button3 0 (`self.CurrentMaterial`))
      (set `self.CurrentValue` 3)
      (set `self.CurrentValueReorder` 3))
    (:`5`
      (`SceneComponent.K2_SetWorldLocation` (`self.SelectedButton`) (`SceneComponent.K2_GetComponentLocation` _button4) false false)
      (`PrimitiveComponent.SetMaterial` `Button N` 0 (`PrimitiveComponent.GetMaterial` _button4 0))
      (`PrimitiveComponent.SetMaterial` _button4 0 (`self.CurrentMaterial`))
      (set `self.CurrentValue` 4)
      (set `self.CurrentValueReorder` 4))))

(fn `ChangeButtonsMaterialsRight`
  (params (`Button N` :type "PrimitiveComponent Object Reference"))
  (bind _button2 (`self.Button2`))
  (bind _button3 (`self.Button3`))
  (bind _button4 (`self.Button4`))
  (bind _button5 (`self.Button5`))
  (bind _button1 (`self.Button1`))
  (switch `int` (`self.CurrentValueReorder`)
    (:`1`
      (`SceneComponent.K2_SetWorldLocation` (`self.SelectedButton`) (`SceneComponent.K2_GetComponentLocation` _button2) false false)
      (`PrimitiveComponent.SetMaterial` `Button N` 0 (`PrimitiveComponent.GetMaterial` _button2 0))
      (`PrimitiveComponent.SetMaterial` _button2 0 (`self.CurrentMaterial`))
      (set `self.CurrentValue` 2)
      (set `self.CurrentValueReorder` 2))
    (:`2`
      (`SceneComponent.K2_SetWorldLocation` (`self.SelectedButton`) (`SceneComponent.K2_GetComponentLocation` _button3) false false)
      (`PrimitiveComponent.SetMaterial` `Button N` 0 (`PrimitiveComponent.GetMaterial` _button3 0))
      (`PrimitiveComponent.SetMaterial` _button3 0 (`self.CurrentMaterial`))
      (set `self.CurrentValue` 3)
      (set `self.CurrentValueReorder` 3))
    (:`3`
      (`SceneComponent.K2_SetWorldLocation` (`self.SelectedButton`) (`SceneComponent.K2_GetComponentLocation` _button4) false false)
      (`PrimitiveComponent.SetMaterial` `Button N` 0 (`PrimitiveComponent.GetMaterial` _button4 0))
      (`PrimitiveComponent.SetMaterial` _button4 0 (`self.CurrentMaterial`))
      (set `self.CurrentValue` 4)
      (set `self.CurrentValueReorder` 4))
    (:`4`
      (`SceneComponent.K2_SetWorldLocation` (`self.SelectedButton`) (`SceneComponent.K2_GetComponentLocation` _button5) false false)
      (`PrimitiveComponent.SetMaterial` `Button N` 0 (`PrimitiveComponent.GetMaterial` _button5 0))
      (`PrimitiveComponent.SetMaterial` _button5 0 (`self.CurrentMaterial`))
      (set `self.CurrentValue` 5)
      (set `self.CurrentValueReorder` 5))
    (:`5`
      (`SceneComponent.K2_SetWorldLocation` (`self.SelectedButton`) (`SceneComponent.K2_GetComponentLocation` _button1) false false)
      (`PrimitiveComponent.SetMaterial` `Button N` 0 (`PrimitiveComponent.GetMaterial` _button1 0))
      (`PrimitiveComponent.SetMaterial` _button1 0 (`self.CurrentMaterial`))
      (set `self.CurrentValue` 1)
      (set `self.CurrentValueReorder` 1))))

(fn `DebugSetMaterial`
  (bind _temparray (`self.TempArray`))
  (`KismetArrayLibrary.Array_Clear` _temparray)
  (`|ExecutionSequence`
    (:`then_0`
      (`KismetArrayLibrary.Array_Add` _temparray (`KismetSystemLibrary.GetObjectName` (`PrimitiveComponent.GetMaterial` (`self.Button1`) 0)))
      (`KismetArrayLibrary.Array_Add` _temparray (`KismetSystemLibrary.GetObjectName` (`PrimitiveComponent.GetMaterial` (`self.Button2`) 0)))
      (`KismetArrayLibrary.Array_Add` _temparray (`KismetSystemLibrary.GetObjectName` (`PrimitiveComponent.GetMaterial` (`self.Button3`) 0)))
      (`KismetArrayLibrary.Array_Add` _temparray (`KismetSystemLibrary.GetObjectName` (`PrimitiveComponent.GetMaterial` (`self.Button4`) 0)))
      (`KismetArrayLibrary.Array_Add` _temparray (`KismetSystemLibrary.GetObjectName` (`PrimitiveComponent.GetMaterial` (`self.Button5`) 0))))
    (:`then_1`
      (for _array_element _temparray
        (`KismetSystemLibrary.PrintString` _array_element true true (struct :`G` 0.66 :`B` 1.0 :`A` 1.0) 20.0))
      (return))))

(fn `GetSelectedButton`
  (returns (ButtonN :type "StaticMeshComponent Object Reference"))
  (switch `int` (`self.CurrentValue`)
    (:`1`
      (return (`self.Button1`)))
    (:`2`
      (return (`self.Button2`)))
    (:`3`
      (return (`self.Button3`)))
    (:`4`
      (return (`self.Button4`)))
    (:`5`
      (return (`self.Button5`)))))

(fn `SetMediaSource`
  (returns (MediaSource :type "MediaSource Object Reference") (MPlay :type "MediaPlayer Object Reference"))
  (locals (SelButton :type "StaticMeshComponent Object Reference"))
  (switch `int` (`self.CurrentValue`)
    (:`1`
      (bind _output_get (set `local.SelButton` (`self.Button1`))))
    (:`2`
      (set `local.SelButton` (`self.Button2`)))
    (:`3`
      (set `local.SelButton` (`self.Button3`)))
    (:`4`
      (set `local.SelButton` (`self.Button4`)))
    (:`5`
      (set `local.SelButton` (`self.Button5`))))
  (switch `string` (`KismetSystemLibrary.GetObjectName` (`PrimitiveComponent.GetMaterial` _output_get 0))
    (:`M_Start4`
      (bind _output_get_2 (set `self.MediaSource` "/Game/Movies/Walking_w_Friends.Walking_w_Friends")))
    (:`M_Start5`
      (set `self.MediaSource` "/Game/Movies/Emily_Funeral.Emily_Funeral"))
    (:`M_Start3`
      (set `self.MediaSource` "/Game/Movies/Tommy_Without_Friends.Tommy_Without_Friends"))
    (:`M_Start2`
      (set `self.MediaSource` "/Game/Movies/Tommy_Emily_Road.Tommy_Emily_Road"))
    (:`M_Start1`
      (set `self.MediaSource` "/Game/Movies/Tommy_Sleeps.Tommy_Sleeps")))
  (return _output_get_2 (`self.MPlay4`)))

(fn `UserConstructionScript`)

(fn `VerifyCombination`
  (returns (ReturnValue :type Boolean))
  (bind _temparray (`self.TempArray`))
  (`KismetArrayLibrary.Array_Clear` _temparray)
  (`|ExecutionSequence`
    (:`then_0`
      (`KismetArrayLibrary.Array_Add` _temparray (`KismetSystemLibrary.GetObjectName` (`PrimitiveComponent.GetMaterial` (`self.Button1`) 0)))
      (`KismetArrayLibrary.Array_Add` _temparray (`KismetSystemLibrary.GetObjectName` (`PrimitiveComponent.GetMaterial` (`self.Button2`) 0)))
      (`KismetArrayLibrary.Array_Add` _temparray (`KismetSystemLibrary.GetObjectName` (`PrimitiveComponent.GetMaterial` (`self.Button3`) 0)))
      (`KismetArrayLibrary.Array_Add` _temparray (`KismetSystemLibrary.GetObjectName` (`PrimitiveComponent.GetMaterial` (`self.Button4`) 0)))
      (`KismetArrayLibrary.Array_Add` _temparray (`KismetSystemLibrary.GetObjectName` (`PrimitiveComponent.GetMaterial` (`self.Button5`) 0))))
    (:`then_1`
      (return (`KismetArrayLibrary.Array_Identical` (`self.TempArray`) (`self.SolutionArray`))))))