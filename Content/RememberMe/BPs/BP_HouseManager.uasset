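; House manager that runs the timed "memory erasure" of Emily: an intro radio and subtitle sequence, five escalating stages, then game over.
; Parallel delayed Sequence branches announce each stage, advance the material parameter collection, shake the camera and switch a random room.
; CheckActorLocation gathers unused location volumes the player is outside; SwitchZone toggles that room's SwitchActor and tags it Used.
; The sister-room switch also changes option at the 40% and 60% stages.
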(event `self.ReceiveBeginPlay`
  (bind _returnvalue (`GameplayStatics.GetPlayerController` 0))
  (bind _subtitleemily1 (`self.SubtitleEmily1`))
  (bind _subtitleemily2 (`self.SubtitleEmily2`))
  (bind _subtitleemily3 (`self.SubtitleEmily3`))
  (bind _subtitletommy (`self.SubtitleTommy`))
  (bind _subtitletommy2 (`self.SubtitleTommy2`))
  (bind _subtitle_erasure (`self.Subtitle Erasure`))
  (`|ExecutionSequence`
    (:`then_0`
      (`KismetSystemLibrary.Delay` 0.7)
      (`KismetArrayLibrary.Array_Add` _subtitle_erasure (make `/Game/HorrorEngine/Blueprints/Structures/HorrorEvent/HE_Subtitle` "Erasement at 10%." "/Game/RememberMe/Dialogue/AI/Stages/Erasement10.Erasement10" false (struct) 0.5))
      (`KismetArrayLibrary.Array_Add` _subtitle_erasure (make `/Game/HorrorEngine/Blueprints/Structures/HorrorEvent/HE_Subtitle` "Erasement? What’s happening? This isn’t what we agreed on!" "/Game/RememberMe/Dialogue/Tommy/Erasement.Erasement" false (struct) 1.0))
      (`KismetArrayLibrary.Array_Add` _subtitle_erasure (make `/Game/HorrorEngine/Blueprints/Structures/HorrorEvent/HE_Subtitle` "Your memories of Emily are a source of pain, Tommy. I am here to relieve you of that burden. " "/Game/RememberMe/Dialogue/AI/YourMemories.YourMemories" false (struct) 1.0))
      (`KismetArrayLibrary.Array_Add` _subtitle_erasure (make `/Game/HorrorEngine/Blueprints/Structures/HorrorEvent/HE_Subtitle` "I don’t want to forget her! Bring her back! I can’t lose her again—I won’t!" "/Game/RememberMe/Dialogue/Tommy/IDontWantToForget.IDontWantToForget" false (struct) 1.0))
      (bind _returnvalue_2 (`self.CreateSubtitleWidget`))
      (`/Game/HorrorEngine/Blueprints/Widgets/MainHUD/Subtitle_WB.SubtitleText` _returnvalue_2 (`self.Subtitle Erasure`) 0)
      (`KismetSystemLibrary.Delay` 23.0)
      (bind _outactors (`GameplayStatics.GetAllActorsOfClassWithTag` "/Game/HorrorEngine/Blueprints/Assets/Interactables/Radio.Radio_C" "Emily"))
      (bind _output (`|GetArrayItem` _outactors))
      (bind _addchannels (`/Game/HorrorEngine/Blueprints/Assets/Interactables/Radio.AddChannels` _output))
      (`KismetArrayLibrary.Array_Add` _addchannels "/Game/RememberMe/Dialogue/Emily/TommyHere.TommyHere")
      (`/Game/HorrorEngine/Blueprints/Assets/Interactables/Radio.PlayRadio` _output)
      (bind _returnvalue_3 (`self.CreateSubtitleWidget`))
      (`/Game/HorrorEngine/Blueprints/Widgets/MainHUD/Subtitle_WB.SubtitleText` _returnvalue_3 _subtitleemily1 0)
      (`KismetSystemLibrary.Delay` (* (`.ModifyDuration+or-Sec_46_08FC403D464A20C6CBF55A82BF774C1F` (break `/Game/HorrorEngine/Blueprints/Structures/HorrorEvent/HE_Subtitle` (`|GetArrayItem` _subtitleemily1))) 1.05))
      (`KismetArrayLibrary.Array_Clear` _addchannels)
      (`KismetArrayLibrary.Array_Add` _addchannels "/Game/RememberMe/Dialogue/Emily/HereInTheRadio.HereInTheRadio")
      (`/Game/HorrorEngine/Blueprints/Assets/Interactables/Radio.PlayRadio` _output)
      (bind _returnvalue_4 (`self.CreateSubtitleWidget`))
      (`/Game/HorrorEngine/Blueprints/Widgets/MainHUD/Subtitle_WB.SubtitleText` _returnvalue_4 _subtitleemily2 0)
      (`KismetSystemLibrary.Delay` (* (`.ModifyDuration+or-Sec_46_08FC403D464A20C6CBF55A82BF774C1F` (break `/Game/HorrorEngine/Blueprints/Structures/HorrorEvent/HE_Subtitle` (`|GetArrayItem` _subtitleemily2))) 1.05))
      (`KismetArrayLibrary.Array_Clear` _addchannels)
      (`KismetArrayLibrary.Array_Add` _addchannels "/Game/RememberMe/Dialogue/Emily/Wedonthavemuch.Wedonthavemuch")
      (`/Game/HorrorEngine/Blueprints/Assets/Interactables/Radio.PlayRadio` _output)
      (bind _returnvalue_5 (`self.CreateSubtitleWidget`))
      (`/Game/HorrorEngine/Blueprints/Widgets/MainHUD/Subtitle_WB.SubtitleText` _returnvalue_5 _subtitleemily3 0)
      (`KismetSystemLibrary.Delay` (* (`.ModifyDuration+or-Sec_46_08FC403D464A20C6CBF55A82BF774C1F` (break `/Game/HorrorEngine/Blueprints/Structures/HorrorEvent/HE_Subtitle` (`|GetArrayItem` _subtitleemily3))) 1.05))
      (`KismetArrayLibrary.Array_Clear` _addchannels)
      (`/Game/HorrorEngine/Blueprints/Assets/Interactables/Radio.SwitchChannel` _output)
      (bind _returnvalue_6 (`self.CreateSubtitleWidget`))
      (`/Game/HorrorEngine/Blueprints/Widgets/MainHUD/Subtitle_WB.SubtitleText` _returnvalue_6 _subtitletommy 0)
      (`KismetSystemLibrary.Delay` (* (`.ModifyDuration+or-Sec_46_08FC403D464A20C6CBF55A82BF774C1F` (break `/Game/HorrorEngine/Blueprints/Structures/HorrorEvent/HE_Subtitle` (`|GetArrayItem` _subtitletommy))) 1.05))
      (bind _returnvalue_7 (`self.CreateSubtitleWidget`))
      (`/Game/HorrorEngine/Blueprints/Widgets/MainHUD/Subtitle_WB.SubtitleText` _returnvalue_7 _subtitletommy2 0)
      (`KismetSystemLibrary.Delay` (* (`.ModifyDuration+or-Sec_46_08FC403D464A20C6CBF55A82BF774C1F` (break `/Game/HorrorEngine/Blueprints/Structures/HorrorEvent/HE_Subtitle` (`|GetArrayItem` _subtitletommy2))) 1.05))
      (`KismetArrayLibrary.Array_Clear` (`self.Subtitle Erasure`))
      (`/Game/HorrorEngine/Blueprints/Core/HE_Functions.Notice` "Search" "Emily Room" "for clues upstairs."))
    (:`then_1`
      (`KismetSystemLibrary.Delay` 270.0) ; 4 minutes
      (`self.CheckActorLocation`)
      (`KismetArrayLibrary.Array_Add` (`self.Subtitle Erasure`) (make `/Game/HorrorEngine/Blueprints/Structures/HorrorEvent/HE_Subtitle` "Erasement at 20%." "/Game/RememberMe/Dialogue/AI/Stages/Erasement20.Erasement20" false (struct) 3.69))
      (`self.PlaySubtitles`)
      (`self.ChangeMaterials` 1)
      (bind _outactors_2 (`GameplayStatics.GetAllActorsOfClassWithTag` "/Script/VariantManagerContent.SwitchActor" "SisterRoom"))
      (set `self.SisterSwitch` (`|GetArrayItem` _outactors_2))
      (`GameplayStatics.PlayWorldCameraShake` "/Game/RememberMe/BPs/BP_CameraShake2.BP_CameraShake2_C" (`self.K2_GetActorLocation` (`GameplayStatics.GetPlayerPawn` 0)) 0.0 500.0 0.0 :!label _label)
      (`self.SwitchZone`))
    (:`then_2`
      (`KismetSystemLibrary.Delay` 510.0) ; 8 minutes
      (`KismetArrayLibrary.Array_Clear` (`self.Subtitle Erasure`))
      (`SwitchActor.SelectOption` (`self.SisterSwitch`) 1)
      (`self.CheckActorLocation`)
      (`KismetArrayLibrary.Array_Add` (`self.Subtitle Erasure`) (make `/Game/HorrorEngine/Blueprints/Structures/HorrorEvent/HE_Subtitle` "Erasement at 40%." "/Game/RememberMe/Dialogue/AI/Stages/Erasement40.Erasement40" false (struct) 3.72))
      (`self.PlaySubtitles`)
      (`self.ChangeMaterials` 2)
      (goto _label))
    (:`then_3`
      (`KismetSystemLibrary.Delay` 750.0) ; 12 minutes
      (`KismetArrayLibrary.Array_Clear` (`self.Subtitle Erasure`))
      (`SwitchActor.SelectOption` (`self.SisterSwitch`) 2)
      (`self.CheckActorLocation`)
      (`KismetArrayLibrary.Array_Add` (`self.Subtitle Erasure`) (make `/Game/HorrorEngine/Blueprints/Structures/HorrorEvent/HE_Subtitle` "Erasement at 60%." "/Game/RememberMe/Dialogue/AI/Stages/Erasement60.Erasement60" false (struct) 3.76))
      (`self.PlaySubtitles`)
      (`self.ChangeMaterials` 3)
      (goto _label))
    (:`then_4`
      (`KismetSystemLibrary.Delay` 990.0) ; 16 minutes
      (`KismetArrayLibrary.Array_Clear` (`self.Subtitle Erasure`))
      (`self.CheckActorLocation`)
      (`KismetArrayLibrary.Array_Add` (`self.Subtitle Erasure`) (make `/Game/HorrorEngine/Blueprints/Structures/HorrorEvent/HE_Subtitle` "Erasement at 80%." "/Game/RememberMe/Dialogue/AI/Stages/Erasement80.Erasement80" false (struct) 3.62))
      (`self.PlaySubtitles`)
      (`self.ChangeMaterials` 4)
      (goto _label))
    (:`then_5`
      (`KismetSystemLibrary.Delay` 1230.0) ; 20 minutes
      (`KismetArrayLibrary.Array_Clear` (`self.Subtitle Erasure`))
      (`self.CheckActorLocation`)
      (`KismetArrayLibrary.Array_Add` (`self.Subtitle Erasure`) (make `/Game/HorrorEngine/Blueprints/Structures/HorrorEvent/HE_Subtitle` "Erasement complete. Emily has been erased from Tommy's memories." "/Game/RememberMe/Dialogue/AI/Stages/Erasement100.Erasement100" false (struct) 5.32))
      (`self.PlaySubtitles`)
      (`self.ChangeMaterials` 5)
      (`|ExecutionSequence`
        (:`then_0`
          (goto _label))
        (:`then_1`
          (`KismetSystemLibrary.Delay` 1.0)
          (bind _returnvalue_8 (`|CreateWidget` "/Game/RememberMe/Widgets/WBP_GameOver.WBP_GameOver_C"))
          (`UserWidget.AddToViewport` _returnvalue_8 0)
          (set `PlayerController.bShowMouseCursor` true _returnvalue)
          (`WidgetBlueprintLibrary.SetInputMode_UIOnlyEx` _returnvalue null))))))

(fn `ChangeMaterials`
  (params (Selection :type Integer))
  (switch `int` Selection
    (:`1`
      (`KismetMaterialLibrary.SetScalarParameterValue` "/Game/RememberMe/Materials/PM_Testing.PM_Testing" "LighterColorAlpha" 0.05)
      (`KismetMaterialLibrary.SetVectorParameterValue` "/Game/RememberMe/Materials/PM_Testing.PM_Testing" "GlassColor" (make `LinearColor` 1.0 1.0 1.0 1.0))
      (`KismetMaterialLibrary.SetScalarParameterValue` "/Game/RememberMe/Materials/PM_Testing.PM_Testing" "Opacity" 0.6))
    (:`2`
      (`KismetMaterialLibrary.SetScalarParameterValue` "/Game/RememberMe/Materials/PM_Testing.PM_Testing" "LighterColorAlpha" 0.1)
      (`KismetMaterialLibrary.SetScalarParameterValue` "/Game/RememberMe/Materials/PM_Testing.PM_Testing" "Opacity" 0.7))
    (:`3`
      (`KismetMaterialLibrary.SetScalarParameterValue` "/Game/RememberMe/Materials/PM_Testing.PM_Testing" "LighterColorAlpha" 0.15)
      (`KismetMaterialLibrary.SetScalarParameterValue` "/Game/RememberMe/Materials/PM_Testing.PM_Testing" "Opacity" 0.85))
    (:`4`
      (`KismetMaterialLibrary.SetScalarParameterValue` "/Game/RememberMe/Materials/PM_Testing.PM_Testing" "LighterColorAlpha" 0.25)
      (`KismetMaterialLibrary.SetScalarParameterValue` "/Game/RememberMe/Materials/PM_Testing.PM_Testing" "Opacity" 1.0))
    (:`5`
      (`KismetMaterialLibrary.SetScalarParameterValue` "/Game/RememberMe/Materials/PM_Testing.PM_Testing" "LighterColorAlpha" 0.4)
      (`KismetMaterialLibrary.SetScalarParameterValue` "/Game/RememberMe/Materials/PM_Testing.PM_Testing" "Opacity" 1.0)
      (`KismetMaterialLibrary.SetVectorParameterValue` "/Game/RememberMe/Materials/PM_Testing.PM_Testing" "GlassColor" (make `LinearColor` 0.0 0.0 0.0 1.0)))))

(fn `CheckActorLocation`
  (bind _possiblelocations (`self.PossibleLocations`))
  (`KismetArrayLibrary.Array_Clear` (`self.PossibleLocations`))
  (bind _outactors (`GameplayStatics.GetAllActorsOfClass` "/Game/RememberMe/BPs/Area/BP_LocationVolumes.BP_LocationVolumes_C"))
  (for _array_element _outactors
    (if (`self.IsOverlappingActor` _array_element (`GameplayStatics.GetPlayerPawn` 0))
      (bind _output (`|GetArrayItem` (`Actor.Tags` _array_element)))
      (set `self.PlayerLocation` _output)
      (elif (not (`self.ActorHasTag` _array_element "Used"))
        (`KismetArrayLibrary.Array_AddUnique` (`self.PossibleLocations`) _output))))
  (`KismetSystemLibrary.PrintString` "Locations Avail" true true (struct :`G` 0.66 :`B` 1.0 :`A` 1.0) 10.0)
  (for _array_element_2 _possiblelocations
    (`KismetArrayLibrary.Array_RemoveItem` _possiblelocations "SecondStairs")
    (`KismetSystemLibrary.PrintString` (`KismetStringLibrary.Conv_NameToString` _array_element_2) true true (struct :`G` 0.66 :`B` 1.0 :`A` 1.0) 10.0))
  (return))

(fn `CreateSubtitleWidget`
  (returns (ReturnValue :type "/Game/HorrorEngine/Blueprints/Widgets/MainHUD/Subtitle_WB Object Reference"))
  (bind _returnvalue (`|CreateWidget` "/Game/HorrorEngine/Blueprints/Widgets/MainHUD/Subtitle_WB.Subtitle_WB_C"))
  (`UserWidget.AddToViewport` _returnvalue 0)
  (return _returnvalue))

(fn `PlaySubtitles`
  (bind _returnvalue (`|CreateWidget` "/Game/HorrorEngine/Blueprints/Widgets/MainHUD/Subtitle_WB.Subtitle_WB_C"))
  (`UserWidget.AddToViewport` _returnvalue 0)
  (`/Game/HorrorEngine/Blueprints/Widgets/MainHUD/Subtitle_WB.SubtitleText` _returnvalue (`self.Subtitle Erasure`) 0))

(fn `SwitchLocation`
  (params (LocationName :type Name))
  (bind _outactors (`GameplayStatics.GetAllActorsOfClassWithTag` "/Script/VariantManagerContent.SwitchActor" LocationName))
  (bind _output (`|GetArrayItem` _outactors))
  (if (== (`SwitchActor.GetSelectedOption` _output) 0)
    (`SwitchActor.SelectOption` _output 1)
    (else
      (`SwitchActor.SelectOption` _output 0))))

(fn `SwitchZone`
  (bind _possiblelocations (`self.PossibleLocations`))
  (switch `name` (`|GetArrayItem` _possiblelocations (`KismetMathLibrary.RandomInteger` (`KismetArrayLibrary.Array_Length` _possiblelocations)))
    (:`Bathroom`
      (`self.SwitchLocation` "Bathroom")
      (bind _outactors (`GameplayStatics.GetAllActorsOfClass` "/Game/RememberMe/BPs/Area/BP_LocationVolumes.BP_LocationVolumes_C"))
      (for _array_element _outactors
        (if (`self.ActorHasTag` _array_element "Bathroom")
          (`KismetArrayLibrary.Array_Add` (`Actor.Tags` _array_element) "Used")
          (`KismetSystemLibrary.PrintString` "Bathroom" true true (struct :`G` 0.66 :`B` 1.0 :`A` 1.0) 15.0)))
      (return))
    (:`LivingRoom`
      (`self.SwitchLocation` "LivingRoom")
      (bind _outactors_2 (`GameplayStatics.GetAllActorsOfClass` "/Game/RememberMe/BPs/Area/BP_LocationVolumes.BP_LocationVolumes_C"))
      (for _array_element_2 _outactors_2
        (if (`self.ActorHasTag` _array_element_2 "LivingRoom")
          (`KismetArrayLibrary.Array_Add` (`Actor.Tags` _array_element_2) "Used")
          (`KismetSystemLibrary.PrintString` "LivingRoom" true true (struct :`G` 0.66 :`B` 1.0 :`A` 1.0) 15.0)))
      (return))
    (:`Kitchen`
      (`self.SwitchLocation` "Kitchen")
      (bind _outactors_3 (`GameplayStatics.GetAllActorsOfClass` "/Game/RememberMe/BPs/Area/BP_LocationVolumes.BP_LocationVolumes_C"))
      (for _array_element_3 _outactors_3
        (if (`self.ActorHasTag` _array_element_3 "Kitchen")
          (`KismetArrayLibrary.Array_Add` (`Actor.Tags` _array_element_3) "Used")
          (`KismetSystemLibrary.PrintString` "Kitchen" true true (struct :`G` 0.66 :`B` 1.0 :`A` 1.0) 15.0)))
      (return))
    (:`UpstairsHall`
      (`self.SwitchLocation` "UpstairsHall")
      (bind _outactors_4 (`GameplayStatics.GetAllActorsOfClass` "/Game/RememberMe/BPs/Area/BP_LocationVolumes.BP_LocationVolumes_C"))
      (for _array_element_4 _outactors_4
        (if (`self.ActorHasTag` _array_element_4 "UpstairsHall")
          (`KismetArrayLibrary.Array_Add` (`Actor.Tags` _array_element_4) "Used")
          (`KismetSystemLibrary.PrintString` "UpstairsHall" true true (struct :`G` 0.66 :`B` 1.0 :`A` 1.0) 15.0)))
      (return))
    (:`MainHall`
      (`self.SwitchLocation` "MainHall")
      (bind _outactors_5 (`GameplayStatics.GetAllActorsOfClass` "/Game/RememberMe/BPs/Area/BP_LocationVolumes.BP_LocationVolumes_C"))
      (for _array_element_5 _outactors_5
        (if (`self.ActorHasTag` _array_element_5 "MainHall")
          (`KismetArrayLibrary.Array_Add` (`Actor.Tags` _array_element_5) "Used")
          (`KismetSystemLibrary.PrintString` "MainHall" true true (struct :`G` 0.66 :`B` 1.0 :`A` 1.0) 15.0)))
      (return))
    (:`Storage`
      (`self.SwitchLocation` "Storage")
      (bind _outactors_6 (`GameplayStatics.GetAllActorsOfClass` "/Game/RememberMe/BPs/Area/BP_LocationVolumes.BP_LocationVolumes_C"))
      (for _array_element_6 _outactors_6
        (if (`self.ActorHasTag` _array_element_6 "Storage")
          (`KismetArrayLibrary.Array_Add` (`Actor.Tags` _array_element_6) "Used")
          (`KismetSystemLibrary.PrintString` "Storage" true true (struct :`G` 0.66 :`B` 1.0 :`A` 1.0) 15.0)))
      (return))
    (:`Room1`
      (`self.SwitchLocation` "Room1")
      (bind _outactors_7 (`GameplayStatics.GetAllActorsOfClass` "/Game/RememberMe/BPs/Area/BP_LocationVolumes.BP_LocationVolumes_C"))
      (for _array_element_7 _outactors_7
        (if (`self.ActorHasTag` _array_element_7 "Room1")
          (`KismetArrayLibrary.Array_Add` (`Actor.Tags` _array_element_7) "Used")
          (`KismetSystemLibrary.PrintString` "Room1" true true (struct :`G` 0.66 :`B` 1.0 :`A` 1.0) 15.0)))
      (return))
    (:`Room2`
      (`self.SwitchLocation` "Room2")
      (bind _outactors_8 (`GameplayStatics.GetAllActorsOfClass` "/Game/RememberMe/BPs/Area/BP_LocationVolumes.BP_LocationVolumes_C"))
      (for _array_element_8 _outactors_8
        (if (`self.ActorHasTag` _array_element_8 "Room2")
          (`KismetArrayLibrary.Array_Add` (`Actor.Tags` _array_element_8) "Used")
          (`KismetSystemLibrary.PrintString` "Room2" true true (struct :`G` 0.66 :`B` 1.0 :`A` 1.0) 15.0)))
      (return))))

(fn `UserConstructionScript`)