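; Moveable door that slides upward once its Activate flag is set and switches on a World Partition data layer as it opens.
; A looping 0.01-second timer, started shortly after BeginPlay, polls the flag, activates the data layer once and raises the mesh a unit per tick until it passes 250 units above its start.
; The mesh's relative X and Y are hardcoded, and the timer is never cleared.
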(event `self.ReceiveBeginPlay`
  (bind (_relativelocation_x _relativelocation_y _relativelocation_z) (`KismetMathLibrary.BreakVector` (`SceneComponent.RelativeLocation` (`self.StaticMeshComponent`))))
  (set `self.MaxZ` (+ _relativelocation_z 250.0))
  (`KismetSystemLibrary.Delay` 0.2)
  (`KismetSystemLibrary.K2_SetTimerDelegate` (delegate `MoveDoor`) 0.01 true))

(event `MoveDoor`
  (bind _staticmeshcomponent (`self.StaticMeshComponent`))
  (bind (_relativelocation_x _relativelocation_y _relativelocation_z) (`KismetMathLibrary.BreakVector` (`SceneComponent.RelativeLocation` _staticmeshcomponent)))
  (if (`self.Activate`)
    (`|ExecutionSequence`
      (:`then_0`
        (`/Engine/EditorBlueprintResources/StandardMacros.DoOnce` false
          (:`Completed`
            (`DataLayerSubsystem.SetDataLayerRuntimeState` (subsystem `DataLayerSubsystem`) (`self.In Data Layer`) "Activated" false))))
      (:`then_1`
        (if (<= _relativelocation_z (`self.MaxZ`))
          (bind _result (`/Engine/EditorBlueprintResources/StandardMacros.IncrementFloat` _relativelocation_z)
            (:`  `
              (`SceneComponent.K2_SetRelativeLocation` _staticmeshcomponent (`KismetMathLibrary.MakeVector` 439.260126 -158.991318 _result) false false))))))))

(fn `UserConstructionScript`)